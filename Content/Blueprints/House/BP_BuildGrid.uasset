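; BP_BuildGrid is an actor that shows the house build grid as a plane that can be toggled visible or hidden.
; Setting visibility also refreshes the plane, which is scaled and centred to cover the map using the House's map size and tile size from the game mode.
; A dynamic instance of MI_BuildGrid receives the tile size as a parameter, so the material's grid follows the house tiles.
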(event Custom|SetGridVisibility
  (params (IsVisible :type Boolean))
  (Rendering|SetVisibility (Variables|Default|GetPlane) IsVisible false)
  (CallFunction|UpdateGridPlane))

(event Custom|UpdateGridPlane
  (bind _returnvalue (Game|GetGameMode))
  (bind _plane (Variables|Default|GetPlane))
  (bind _asiggame_mode (Utilities|Casting|CastToIGGameMode _returnvalue))
  (bind _returnvalue_2 (Class|IGGameMode|GetHouse _asiggame_mode))
  (bind _returnvalue_3 (Class|House|GetMapSize _returnvalue_2))
  (bind _returnvalue_4 (Class|House|GetTileSize _returnvalue_2))
  (bind _returnvalue_5 (* _returnvalue_3 _returnvalue_4))
  (bind _returnvalue_6 (/ _returnvalue_5 2.0))
  (bind _returnvalue_7 (/ _returnvalue_5 1e+02))
  (bind _returnvalue_8 (Rendering|Material|CreateDynamicMaterialInstance (Variables|Default|GetPlane) 0 "/Game/Materials/MI_BuildGrid.MI_BuildGrid" "None" :!class /Script/Engine.PrimitiveComponent))
  (Rendering|Material|SetScalarParameterValue _returnvalue_8 "TileSize" _returnvalue_4 :!class /Script/Engine.MaterialInstanceDynamic)
  (Transformation|SetWorldScale3D _plane (Math|Vector|MakeVector _returnvalue_7 _returnvalue_7 1.0))
  (Transformation|SetWorldLocation _plane (Math|Vector|MakeVector _returnvalue_6 _returnvalue_6 2.0) false false))

(fn ConstructionScript)