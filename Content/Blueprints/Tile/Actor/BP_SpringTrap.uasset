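; BP_SpringTrap is a tile-based spring trap actor that toggles its Cone component's visibility as actors move across it.
; On entry it calls the parent handler and shows the cone.
; On leave it calls the parent handler, then keeps the cone visible only if the destination tile, offset from the trap's tile position, lies within its tiled model.
; No triggering or spring effect is implemented in this graph.
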(event EventBeginPlay)

(event Collision|EventActorBeginOverlap
  (params (OtherActor :type Actor%20Object%20Reference)))

(event EventTick
  (params (DeltaSeconds :type Float%20%28single-precision%29)))

(event EventOnActorEntered
  (params (EnteringActor :type Actor%20Object%20Reference) (FromTile :type Int%20Point%20Structure%20%28by%20ref%29))
  (|CallParentFunction EnteringActor FromTile)
  (Rendering|SetVisibility (Variables|Default|GetCone) true false))

(event EventOnActorLeave
  (params (LeavingActor :type Actor%20Object%20Reference) (ToTile :type Int%20Point%20Structure%20%28by%20ref%29))
  (bind (_x _y) (Utilities|Struct|BreakIntPoint ToTile))
  (bind _returnvalue (Class|TileActor|GetTilePos))
  (|CallParentFunction LeavingActor ToTile)
  (Rendering|SetVisibility (Variables|Default|GetCone) (Utilities|Array|ContainsItem (Class|TileActor|GetTiledModel) (Utilities|Struct|MakeIntPoint (- _x (.x _returnvalue)) (- _y (.y _returnvalue)))) false))

(fn ConstructionScript)